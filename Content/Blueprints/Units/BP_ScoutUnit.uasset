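; BP_ScoutUnit is a scout unit Blueprint that handles the unit's audio feedback.
; Movement component start and end events unpause and pause a looping-style movement sound, which starts paused.
; Tick mutes that sound whenever the actor is hidden.
; Destruction plays an attenuated defeat sound at its location, and returning to HQ plays a 2D scout sound.
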(event `self.ReceiveBeginPlay`
  (bind _movementcomponent (`self.MovementComponent`))
  (`AudioComponent.SetPaused` (`self.MovementSound`) true)
  (add `UnitMovementComponent.OnMovementStart` _movementcomponent (delegate `On Movement Start`))
  (add `UnitMovementComponent.OnMovementEnd` _movementcomponent (delegate `On Movement End`)))

(event `On Movement Start`
  (`AudioComponent.SetPaused` (`self.MovementSound`) false))

(event `On Movement End`
  (`AudioComponent.SetPaused` (`self.MovementSound`) true))

(event `self.ReceiveDestroyed`
  (`GameplayStatics.PlaySoundAtLocation` "/Game/Audio/Sounds/GlobalMap/Unit/Scout/SW_ScoutDefeat.SW_ScoutDefeat" (`self.K2_GetActorLocation`) (struct) 1.0 1.0 0.0 "/Game/Audio/Sounds/GlobalMap/Unit/SA_Units.SA_Units" null null null))

(event `self.OnReturnToHQ`
  (`GameplayStatics.PlaySound2D` "/Game/Audio/Sounds/HQ/SW_Scout.SW_Scout" 1.0 1.0 0.0 null null))

(event `self.ReceiveTick`
  (params (DeltaSeconds :type "Float (single-precision)"))
  (bind _movementsound (`self.MovementSound`))
  (if (`self.bHidden`)
    (`AudioComponent.SetVolumeMultiplier` _movementsound 0.0)
    (else
      (`AudioComponent.SetVolumeMultiplier` _movementsound 1.0))))

(fn `UserConstructionScript`)