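; BP_CombatUnit is a battlefield unit shown as six meshes, configured from its CombatUnitData asset.
; Data changes apply the mesh and transform, and pick an infantry, cavalry or artillery movement sound.
; Tick hides meshes as CombatComponent health drops, pauses sound when stationary, and mutes it when hidden.
; When French infantry is destroyed and BP_Tutorial exists, a tally of such units can trigger the tutorial's EnemyDefeat.
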(event `self.OnCombatUnitDataChange`
  (bind _combatunitstats_unittype (break `CombatUnitStats` (`CombatUnitDataAsset.CombatUnitStats` (`self.CombatUnitData`))))
  (`|ExecutionSequence` :!label _label
    (:`then_0`
      (`/Engine/EditorBlueprintResources/StandardMacros.IsValid` (`CombatUnitDataAsset.UnitMesh` (`self.CombatUnitData`))
        (:`Is Valid`
          (`self.Set Unit Mesh` (`self.Cube`))
          (`self.Set Unit Mesh` (`self.Cube1`))
          (`self.Set Unit Mesh` (`self.Cube2`))
          (`self.Set Unit Mesh` (`self.Cube3`))
          (`self.Set Unit Mesh` (`self.Cube4`))
          (`self.Set Unit Mesh` (`self.Cube5`)))))
    (:`then_1`
      (switch `ECombatUnitType` _combatunitstats_unittype
        (:`Infantry`
          (`AudioComponent.SetSound` (`self.MovementSound`) "/Game/Audio/Sounds/GlobalMap/Unit/Infantry/SW_InfantryMove.SW_InfantryMove"))
        (:`Cavalry`
          (`AudioComponent.SetSound` (`self.MovementSound`) "/Game/Audio/Sounds/GlobalMap/Unit/Cavalty/SW_CavalryMove.SW_CavalryMove"))
        (:`Artillery`
          (`AudioComponent.SetSound` (`self.MovementSound`) "/Game/Audio/Sounds/GlobalMap/Unit/Artillery/SW_ArtilleryMove.SW_ArtilleryMove"))))
    (:`then_2`
      (`AudioComponent.Play` (`self.MovementSound`) 0.0))))

(event `self.ReceiveBeginPlay`
  (`AudioComponent.SetPaused` (`self.MovementSound`) true)
  (`/Engine/EditorBlueprintResources/StandardMacros.IsValid` (`self.CombatUnitData`)
    (:`Is Valid`
      (goto _label))))

(event `self.ReceiveTick`
  (params (DeltaSeconds :type "Float (single-precision)"))
  (bind _movementsound (`self.MovementSound`))
  (bind _healthpoints (`UnitCombatComponent.HealthPoints` (`self.CombatComponent`)))
  (`|ExecutionSequence`
    (:`then_0`
      (`SceneComponent.SetVisibility` (`self.Cube5`) (< 800.0 _healthpoints) false)
      (`SceneComponent.SetVisibility` (`self.Cube4`) (< 600.0 _healthpoints) false)
      (`SceneComponent.SetVisibility` (`self.Cube3`) (< 400.0 _healthpoints) false)
      (`SceneComponent.SetVisibility` (`self.Cube2`) (< 200.0 _healthpoints) false)
      (`SceneComponent.SetVisibility` (`self.Cube1`) (< 100.0 _healthpoints) false)
      (`SceneComponent.SetVisibility` (`self.Cube`) (< 0.0 _healthpoints) false))
    (:`then_1`
      (`AudioComponent.SetPaused` _movementsound (not (`UnitMovementComponent.bIsMoving` (`self.MovementComponent`))))
      (if (`self.bHidden`)
        (`AudioComponent.SetVolumeMultiplier` _movementsound 0.0)
        (else
          (`AudioComponent.SetVolumeMultiplier` _movementsound 1.0))))))

(event `self.ReceiveDestroyed`
  (if (== (`self.CombatUnitData`) "/Game/Data/Units/FrenchEmpireUnits/DA_FrenchInfantry.DA_FrenchInfantry")
    (bind _returnvalue (`GameplayStatics.GetActorOfClass` "/Game/Blueprints/BP_Tutorial.BP_Tutorial_C"))
    (`/Engine/EditorBlueprintResources/StandardMacros.IsValid` _returnvalue
      (:`Is Valid`
        (bind _outactors (`GameplayStatics.GetAllActorsOfClass` "BP_CombatUnit_C"))
        (for _array_element _outactors
          (if (== (`CombatUnit.CombatUnitData` _array_element) "/Game/Data/Units/FrenchEmpireUnits/DA_FrenchInfantry.DA_FrenchInfantry")
            (`/Engine/EditorBlueprintResources/StandardMacros.DecrementInt` (`self.AllFrenchArmy`))))
        (if (== (`self.AllFrenchArmy`) 1)
          (`/Game/UI/Widgets/Unsorted/WB_Tutorial.EnemyDefeat` (`/Game/Blueprints/BP_Tutorial.Tutorial` _returnvalue)))))))

(fn `Set Unit Mesh`
  (params (Component :type "StaticMeshComponent Object Reference"))
  (bind _combatunitdata (`self.CombatUnitData`))
  (bind (_unitmeshtransform_location _unitmeshtransform_rotation _unitmeshtransform_scale) (`KismetMathLibrary.BreakTransform` (`CombatUnitDataAsset.UnitMeshTransform` _combatunitdata)))
  (`StaticMeshComponent.SetStaticMesh` Component (`CombatUnitDataAsset.UnitMesh` _combatunitdata))
  (`SceneComponent.K2_AddRelativeLocation` Component _unitmeshtransform_location false false)
  (`SceneComponent.K2_AddRelativeRotation` Component _unitmeshtransform_rotation false false)
  (`SceneComponent.SetRelativeScale3D` Component _unitmeshtransform_scale))

(fn `UserConstructionScript`)