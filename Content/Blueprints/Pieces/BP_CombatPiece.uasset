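; BP_CombatPiece is a game piece actor whose graphs handle its audio feedback.
; A PlaySound event maps a sound type to drag, select or death sounds played at the piece's location.
; Hit plays a placement sound only for impacts above a squared impulse threshold, and ignores hits during the first second of game time.
; The construction script is empty, with an unconnected mesh setter left in it.
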(event `self.PlaySound`
  (params (SoundType :type "EPieceSoundType Enum" :default "StartDragging"))
  (bind _returnvalue (`self.K2_GetActorLocation`))
  (switch `EPieceSoundType` SoundType
    (:`StartDragging`
      (`GameplayStatics.PlaySoundAtLocation` "/Game/Audio/Sounds/Piece/SW_Drag.SW_Drag" _returnvalue (struct) 1.0 1.0 0.0 null null null null))
    (:`Selected`
      (`GameplayStatics.PlaySoundAtLocation` "/Game/Audio/Sounds/Piece/SW_Select.SW_Select" _returnvalue (struct) 1.0 1.0 0.0 null null null null))
    (:`Death`
      (`GameplayStatics.PlaySoundAtLocation` "/Game/Audio/Sounds/Piece/SW_Death.SW_Death" _returnvalue (struct) 1.0 1.0 0.0 null null null null))))

(event `self.ReceiveHit`
  (params (MyComp :type "PrimitiveComponent Object Reference") (Other :type "Actor Object Reference") (OtherComp :type "PrimitiveComponent Object Reference") (bSelfMoved :type Boolean) (HitLocation :type "Vector Structure") (HitNormal :type "Vector Structure") (NormalImpulse :type "Vector Structure") (Hit :type "HitResult Structure (by ref)"))
  (if (> (`GameplayStatics.GetTimeSeconds`) 1.0)
    (if (> (`KismetMathLibrary.VSizeSquared` NormalImpulse) (`KismetMathLibrary.MultiplyMultiply_FloatFloat` 5000.0 2.0))
      (`GameplayStatics.PlaySoundAtLocation` "/Game/Audio/Sounds/Piece/SW_Place.SW_Place" (`self.K2_GetActorLocation`) (struct) 1.0 1.0 0.0 null null null null))))

(fn `UserConstructionScript`)