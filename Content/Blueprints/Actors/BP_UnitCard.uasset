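; BP_UnitCard is an actor that presents a combat unit as spawned pieces plus a widget card.
; On BeginPlay it passes its CombatUnitData and Amount to a child-actor PiecesSpawner and tells it to spawn the pieces.
; It then initializes the UW_UnitCard widget in its widget component with the same unit data.
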(event `self.ReceiveBeginPlay`
  (`|ExecutionSequence`
    (:`then_0`
      (bind _aspieces_spawner (cast `PiecesSpawner` (`ChildActorComponent.ChildActor` (`self.PiecesSpawner`))))
      (set `PiecesSpawner.CombatUnitData` (`self.Combat Unit Data`) _aspieces_spawner)
      (set `PiecesSpawner.Amount` (`self.Amount`) _aspieces_spawner)
      (`PiecesSpawner.SpawnPieces` _aspieces_spawner))
    (:`then_1`
      (bind _asuw_unit_card (cast `/Game/UI/Widgets/UnitCard/UW_UnitCard` (`WidgetComponent.GetWidget` (`self.Widget`))))
      (`/Game/UI/Widgets/UnitCard/UW_UnitCard.Init` _asuw_unit_card (`self.Combat Unit Data`)))))

(fn `UserConstructionScript`)