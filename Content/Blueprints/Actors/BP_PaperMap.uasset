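; BP_PaperMap is a paper map actor that tells the tutorial when a combat or scout piece overlaps it.
; BeginPlay raises the paper mesh's translucent sort priority, then after a short delay finds BP_Tutorial and caches its Tutorial reference.
; The Box overlap casts the entering actor to CombatPiece or ScoutPiece and calls the matching map-overlap function on that Tutorial, if valid.
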(event `self.ReceiveBeginPlay`
  (`PrimitiveComponent.SetTranslucentSortPriority` (`self.PaperMeshComponent`) 5)
  (`KismetSystemLibrary.Delay` 1.0)
  (bind _returnvalue (`GameplayStatics.GetActorOfClass` "/Game/Blueprints/BP_Tutorial.BP_Tutorial_C"))
  (`/Engine/EditorBlueprintResources/StandardMacros.IsValid` _returnvalue
    (:`Is Valid`
      (bind _tutorial (`/Game/Blueprints/BP_Tutorial.Tutorial` _returnvalue))
      (`/Engine/EditorBlueprintResources/StandardMacros.IsValid` _tutorial
        (:`Is Valid`
          (set `self.Tutorial` _tutorial))))))

(event `self.Box.OnComponentBeginOverlap`
  (params (OverlappedComponent :type "PrimitiveComponent Object Reference") (OtherActor :type "Actor Object Reference") (OtherComp :type "PrimitiveComponent Object Reference") (OtherBodyIndex :type Integer) (bFromSweep :type Boolean) (SweepResult :type "HitResult Structure (by ref)"))
  (`/Engine/EditorBlueprintResources/StandardMacros.IsValid` (stale `self.ReceiveBeginPlay` _returnvalue)
    (:`Is Valid`
      (cast `CombatPiece` OtherActor
        (:`then`
          (bind _tutorial (`/Game/Blueprints/BP_Tutorial.Tutorial` (stale `self.ReceiveBeginPlay` _returnvalue)))
          (`/Engine/EditorBlueprintResources/StandardMacros.IsValid` _tutorial
            (:`Is Valid`
              (`/Game/UI/Widgets/Unsorted/WB_Tutorial.CombatMapOvelap` _tutorial))))
        (:`CastFailed`
          (cast `ScoutPiece` OtherActor)
          (`/Engine/EditorBlueprintResources/StandardMacros.IsValid` _tutorial
            (:`Is Valid`
              (`/Game/UI/Widgets/Unsorted/WB_Tutorial.ScoutMapOvelap` _tutorial))))))))

(fn `UserConstructionScript`)