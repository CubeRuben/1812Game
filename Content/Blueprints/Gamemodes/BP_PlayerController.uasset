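; Player controller that handles the pause menu and has placeholder hooks for a gameplay HUD and timer.
; The PauseMenu input creates the pause widget on first use, reuses it afterwards, adds it to the viewport and pauses the game.
; BeginPlay calls CreateHUD and UpdateTimer, but both events are empty.
; The HUD creation, timer formatting, unit card and UI-only input nodes are disconnected and never run.
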(event `self.ReceiveBeginPlay`
  (`self.CreateHUD`)
  (`self.UpdateTimer` 0))

(event `UpdateTimer`
  (params (Timer :type Integer))
  ;[1 1 1] Timer
)

(event `InputAction|PauseMenu`
  (params (Key :type "Key Structure"))
  ;[1 1 1] Pause the game
  (:`Pressed`
    (`/Engine/EditorBlueprintResources/StandardMacros.IsValid` (`self.PauseMenuRef`)
      (:`Is Valid`
        _)
      (:`Is Not Valid`
        (bind _returnvalue (`|CreateWidget` "/Game/UI/Widgets/Unsorted/WB_PauseMenu.WB_PauseMenu_C"))
        (bind _output_get (set `self.PauseMenuRef` _returnvalue))))
    (`UserWidget.AddToViewport` _output_get 0)
    (`GameplayStatics.SetGamePaused` true)))

(event `CreateHUD`
  ;[1 1 1] Create HUD in Gameplay
)

(event `Key|RightMouseButton`
  (params (Key :type "Key Structure")))

(fn `UserConstructionScript`)